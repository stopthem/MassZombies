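; Crowd actor that fills an instanced static mesh with a grid of animated characters using AnimToTexture.
; The construction script places Rows by Columns instances with seeded random X shuffle and yaw.
; Each instance gets a random animation state from the data asset, written to per-instance custom data as frame range, play rate, looping and random time offset.
; Event graph is empty; the AnimToTexture instance-data helper nodes are unconnected.
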(event EventBeginPlay)

(event Collision|EventActorBeginOverlap
  (params (OtherActor :type Actor%20Object%20Reference)))

(event EventTick
  (params (DeltaSeconds :type Float%20%28single-precision%29)))

(fn ConstructionScript
  (bind _randomstream (Variables|Default|GetRandomStream))
  (bind _instancedstaticmesh (Variables|Default|GetInstancedStaticMesh))
  (bind _dataasset (Variables|Default|GetDataAsset))
  (bind _randomstream_2 (Variables|Default|GetRandomStream))
  (bind _maxangle (Variables|Default|GetMaxAngle))
  (bind _animations (Variables|/Script/AnimToTexture.AnimToTextureDataAsset|GetAnimations _dataasset))
  (bind _returnvalue (Utilities|Array|Length _animations))
  (bind _returnvalue_2 (- _returnvalue 1))
  (bind _returnvalue_3 (Math|Random|RandomIntegerinRangefromStream 0 _returnvalue_2 _randomstream))
  ;[1 1 1] Comment
  (Utilities|FlowControl|Sequence
    (:then_0
      (Components|StaticMesh|SetStaticMesh (Variables|Default|GetInstancedStaticMesh) (Variables|Default|GetStaticMeshAsset)))
    (:then_1
      (for _index (range 0 (- (Variables|Default|GetRows) 1))
        (for _index_2 (range 0 (- (Variables|Default|GetColumns) 1))
          (Components|InstancedStaticMesh|AddInstance (Variables|Default|GetInstancedStaticMesh) (Math|Transform|MakeTransform (Math|Vector|MakeVector (+ (* _index_2 (Variables|Default|GetColDistance)) (Math|Random|RandomFloatinRangefromStream 0.0 (Variables|Default|GetShuffleAmount) _randomstream_2)) (* _index (Variables|Default|GetRowDistance)) 0.0) (Math|Rotator|MakeRotator 0.0 0.0 (Math|Random|RandomFloatinRangefromStream (* _maxangle -1.0) _maxangle _randomstream_2))) false))))
    (:then_2
      (for _index_3 (range 0 (- (* (Variables|Default|GetRows) (Variables|Default|GetColumns)) 1))
        (bind _output_get (Variables|Default|SetStruct%20Ref (.AnimState (Class|AnimtoTextureInstancePlaybackLibrary|AnimStatefromDataAsset (Variables|Default|GetDataAsset) _returnvalue_3))))
        ;;[1 1 1] Frame Offset [0]
        (Components|InstancedStaticMesh|SetCustomDataValue _instancedstaticmesh _index_3 0 (.StartFrame (Utilities|Struct|BreakAnimToTextureAnimState _output_get)) false)
        ;;[1 1 1] NumFrames [1]
        (Components|InstancedStaticMesh|SetCustomDataValue _instancedstaticmesh _index_3 1 (.NumFrames (Utilities|Struct|BreakAnimToTextureAnimState _output_get)) false)
        ;;[1 1 1] Playrate [2]
        (Components|InstancedStaticMesh|SetCustomDataValue _instancedstaticmesh _index_3 2 1.0 false)
        ;;[1 1 1] Looping [3]
        (Components|InstancedStaticMesh|SetCustomDataValue _instancedstaticmesh _index_3 3 (.bLooping (Utilities|Struct|BreakAnimToTextureAnimState _output_get)) false)
        ;;[1 1 1] TimeStartOffset [4] (rand value)
        (Components|InstancedStaticMesh|SetCustomDataValue _instancedstaticmesh _index_3 4 (* (Math|Random|RandomFloatfromStream (Variables|Default|GetRandomStream)) (Variables|Default|GetTimeOffsetGain)) false)
        (Utilities|Struct|SetmembersinAnimToTextureAnimState (Variables|Default|GetStruct%20Ref) 0.0 6e+01 1.0)
        (if (Variables|Default|GetPrintDebug)
          (Development|PrintString (Utilities|String|ToString(Text) (Utilities|Text|FormatText " 
InstIndex: {index} 
NumFrames: {NumFrames} 
StartFrame:  {StartFrame} 
PlayRate: {PlayRate} 
BLooping: {BLoopint} 
GlobalStartTime: {GlobalStartTime} 
AnimIndex: {randInt} 
NumMotions: {motionsLen} 
++++++++++++++++++++++" _index_3 (.NumFrames (Utilities|Struct|BreakAnimToTextureAnimState _output_get)) (.StartFrame (Utilities|Struct|BreakAnimToTextureAnimState _output_get)) (.PlayRate (Utilities|Struct|BreakAnimToTextureAnimState _output_get)) (.bLooping (Utilities|Struct|BreakAnimToTextureAnimState _output_get)) (.GlobalStartTime (Utilities|Struct|BreakAnimToTextureAnimState _output_get)) _returnvalue_3 _returnvalue))))))))